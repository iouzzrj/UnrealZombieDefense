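; BP_Character is a player-controlled character with world-axis movement and mouse-aimed facing, in the style of a top-down game.
; BeginPlay caches the PlayerController and adds the default Enhanced Input mapping context.
; IA_Move maps input to fixed world X and Y axes, independent of facing.
; IA_Look intersects the deprojected mouse ray with the Z=0 plane and sets control rotation yaw toward that point.
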(event `self.ReceiveBeginPlay`
  (bind _asplayer_controller (cast `PlayerController` (`self.GetController`)))
  (bind _output_get (set `self.As Player Controller` _asplayer_controller))
  (bind _returnvalue (pcsubsystem `EnhancedInputLocalPlayerSubsystem` _output_get))
  (`/Engine/EditorBlueprintResources/StandardMacros.IsValid` _returnvalue
    (:`Is Valid`
      (`EnhancedInputSubsystemInterface.AddMappingContext` _returnvalue "/Game/Input/IMC_Default.IMC_Default" 0 (struct)))))

(event `EnhancedInput|/Game/Input/IA_Move`
  (params (ActionValue :type "Vector2D Structure") (ElapsedSeconds :type "Float (double-precision)") (TriggeredSeconds :type "Float (double-precision)") (InputAction :type "InputAction Object Reference" :default "/Game/Input/IA_Move.IA_Move"))
  (bind (_x _y) (`KismetMathLibrary.BreakVector2D` ActionValue))
  (:`Triggered`
    ;[1 1 1] 需要将手柄XY轴映射到世界XY轴
    (`self.AddMovementInput` (0.0 1.0 0.0) _x) ; 左右移动
    (`self.AddMovementInput` (1.0 -0.0 0.0) _y) ; 前后移动
  ))

(event `EnhancedInput|/Game/Input/IA_Look`
  (params (ActionValue :type "Vector2D Structure") (ElapsedSeconds :type "Float (double-precision)") (TriggeredSeconds :type "Float (double-precision)") (InputAction :type "InputAction Object Reference" :default "/Game/Input/IA_Look.IA_Look"))
  (bind (_worldlocation _worlddirection) (`PlayerController.DeprojectMousePositionToWorld` (`self.As Player Controller`)))
  (:`Triggered`
    ;[1 1 1] 计算并设定人物所需转向角度
    (`Controller.SetControlRotation` (`self.As Player Controller`) (`KismetMathLibrary.MakeRotator` 0.0 0.0 (.yaw (`KismetMathLibrary.FindLookAtRotation` (`self.K2_GetActorLocation`) (+ _worldlocation (* _worlddirection (/ (* (.z _worldlocation) -1.0) (.z _worlddirection))))))))))

(fn `UserConstructionScript`)